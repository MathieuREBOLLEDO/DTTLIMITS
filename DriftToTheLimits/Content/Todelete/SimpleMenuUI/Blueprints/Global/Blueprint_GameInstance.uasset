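; Game instance that acts as the global hub for menus, settings, singleplayer save slots and multiplayer sessions.
; Menu widgets are created on first show and cached, and session, network and travel failures open an error dialog.
; Settings and level slots persist through SaveGame objects, with a missing settings file saved then reloaded.
; Loaded settings apply volumes via sound mix overrides and rebuild input mappings at runtime from saved key bindings.
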(event `Save Settings`
  ;[1 1 1] Save Settings
  (`self.Save Game Object`))

(event `Load Settings`
  ;[1 1 1] Loading Settings
  (bind _returnvalue (`self.Load Game Object` (`self.GameObjectSlot`)))
  (bind _asgame_object_settings_save_file (cast `/Game/Todelete/SimpleMenuUI/Blueprints/SaveFiles/GameObject_SettingsSaveFile` _returnvalue)
    (:`then`
      (set `self.GameplayInfo` (`/Game/Todelete/SimpleMenuUI/Blueprints/SaveFiles/GameObject_SettingsSaveFile.GameplayInfo` _asgame_object_settings_save_file))
      (set `self.AdvancedGraphicsInfo` (`/Game/Todelete/SimpleMenuUI/Blueprints/SaveFiles/GameObject_SettingsSaveFile.GraphicsInfo` _asgame_object_settings_save_file))
      (bind _output_get (set `self.AudioInfo` (`/Game/Todelete/SimpleMenuUI/Blueprints/SaveFiles/GameObject_SettingsSaveFile.AudioInfo` _asgame_object_settings_save_file)))
      (bind (_mastervolume _sfxvolume _dialogvolume _soundtrackvolume _ambientvolume) (break `/Game/Todelete/SimpleMenuUI/Blueprints/Global/Struct_AudioInfo` _output_get))
      (`self.Apply Audio Setting` _mastervolume _sfxvolume _dialogvolume _soundtrackvolume _ambientvolume)
      (bind _structout (setmembers `/Game/Todelete/SimpleMenuUI/Blueprints/Global/Struct_PlayerInfo` :`StructRef` (make `/Game/Todelete/SimpleMenuUI/Blueprints/Global/Struct_PlayerInfo` (`KismetTextLibrary.Conv_StringToText` (`PlayerState.GetPlayerName` (`Controller.PlayerState` (`GameplayStatics.GetPlayerController` 0)))))))
      (set `self.PlayerInfo` _structout)
      (bind (_moveforward _moveright _jump _invertmousey _fire _dashaction _hat _crouch _weaponmode _cancelhat) (break `/Game/Todelete/SimpleMenuUI/Blueprints/Global/Struct_ControlInfo` (`/Game/Todelete/SimpleMenuUI/Blueprints/SaveFiles/GameObject_SettingsSaveFile.ControlInfo` _asgame_object_settings_save_file)))
      (`self.Set Control Info` _moveforward _moveright _jump _invertmousey _fire _dashaction _hat _crouch _weaponmode _cancelhat))
    (:`CastFailed`
      (`self.Save Game Object`)
      (`self.Load Settings`))))

(event `Start Example Level`
  ;[1 1 1] Start Example Level - Only Used for singleplayer
  (bind _returnvalue (`KismetArrayLibrary.Array_Add` (`self.SingleplayerSlotsInfo`) (make `/Game/Todelete/SimpleMenuUI/Blueprints/Global/Struct_SingleplayerSlot` "PersistentProto" "0.000000,0.000000,0.000000|0.000000,0.000000,-0.000000|1.000000,1.000000,1.000000" (`KismetMathLibrary.UtcNow`))))
  (set `self.LastUsedSingleplayerSlotIDX` _returnvalue)
  (`self.Save Singleplayer Slots`)
  (`WidgetLayoutLibrary.RemoveAllWidgets`)
  (`GameplayStatics.OpenLevel` "PersistentProto")
  (set `self.InGame` true))

(event `Show Opening Widget`
  ;[0 0.5457 1 1 42] Widegts & Menu Items
  ;;[1 1 1] Show Opening Screen
  (if (`self.WasStartScreenShown`)
    (`self.Show Main Menu`)
    (else
      (`self.Show Start Screen`))))

(event `Launch Lobby`
  (params (`Public Connections` :type Integer))
  ;[1 0.09167 0 1 42] Multiplayer Only Events
  ;;[1 1 1] Launch Lobby
  (`self.Show Loading Screen`)
  (set `self.Server Name` (`self.Generate Server Name`))
  (bind _output_get (set `self.Max Connections` `Public Connections`))
  (`CreateSessionCallbackProxy.CreateSession` (`GameplayStatics.GetPlayerController` 0) _output_get
    (:`OnSuccess`
      (set `self.InGame` true)
      (`GameplayStatics.OpenLevel` "Level_Lobby" true "listen"))
    (:`OnFailure`
      (`self.DisplayErrorMessage` "Failed to create session"))))

(event `Load Level`
  (params (IDX :type Integer) (LevelName :type Name))
  ;[1 1 1] Start Example Level - Only Used for singleplayer
  (set `self.LastUsedSingleplayerSlotIDX` IDX)
  (`self.Save Singleplayer Slots`)
  (`WidgetLayoutLibrary.RemoveAllWidgets`)
  (`GameplayStatics.OpenLevel` LevelName)
  (set `self.InGame` true))

(event `Show Start Screen`
  (bind _returnvalue (`GameplayStatics.GetPlayerController` 0))
  ;[0 0.5457 1 1 42] Widegts & Menu Items
  ;;[1 1 1] Show Start Screen
  (`/Engine/EditorBlueprintResources/StandardMacros.IsValid` (`self.StartScreen`)
    (:`Is Valid`
      _)
    (:`Is Not Valid`
      (bind _returnvalue_2 (`|CreateWidget` "/Game/Todelete/SimpleMenuUI/UI/Widgets/MenuWidgets/Widget_StartScreen.Widget_StartScreen_C" _returnvalue))
      (bind _output_get (set `self.StartScreen` _returnvalue_2))))
  (`UserWidget.AddToViewport` _output_get 0)
  (set `PlayerController.bShowMouseCursor` false _returnvalue)
  (set `self.WasStartScreenShown` true))

(event `Join Session`
  (params (Session :type "BlueprintSessionResult Structure"))
  ;[1 0.09167 0 1 42] Multiplayer Only Events
  ;;[1 1 1] Join Session
  (`self.Show Loading Screen`)
  (`JoinSessionCallbackProxy.JoinSession` (`GameplayStatics.GetPlayerController` 0) Session
    (:`OnSuccess`
      (set `self.InGame` true))
    (:`OnFailure`
      (`self.DisplayErrorMessage` "Failed to join server"))))

(event `Show Main Menu`
  (bind _returnvalue (`GameplayStatics.GetPlayerController` 0))
  ;[0 0.5457 1 1 42] Widegts & Menu Items
  ;;[1 1 1] Show Main Menu
  (`/Engine/EditorBlueprintResources/StandardMacros.IsValid` (`self.MainMenu`)
    (:`Is Valid`
      _)
    (:`Is Not Valid`
      (bind _returnvalue_2 (`|CreateWidget` "/Game/Todelete/SimpleMenuUI/UI/Widgets/MenuWidgets/Widget_MainMenu.Widget_MainMenu_C" _returnvalue))
      (bind _output_get (set `self.MainMenu` _returnvalue_2))))
  (`UserWidget.AddToViewport` _output_get 0)
  (set `PlayerController.bShowMouseCursor` true _returnvalue)
  (`WidgetBlueprintLibrary.SetInputMode_UIOnlyEx` _returnvalue _output_get)
  (set `self.InGame` false))

(event `Destroy Session Caller`
  (params (`Player Controller` :type "PlayerController Object Reference"))
  ;[1 0.09167 0 1 42] Multiplayer Only Events
  ;;[1 1 1] Destroy Session Caller
  (`DestroySessionCallbackProxy.DestroySession` `Player Controller`))

(event `self.HandleNetworkError`
  (params (FailureType :type "ENetworkFailure Enum" :default "NetDriverAlreadyExists") (bIsServer :type Boolean))
  ;[1 0.09167 0 1 42] Multiplayer Only Events
  ;;[1 1 1] On Network Error
  (`self.DisplayErrorMessage` (`|GetEnumeratorNameAsString` FailureType)))

(event `Show Singleplayer Menu`
  ;[0 0.5457 1 1 42] Widegts & Menu Items
  ;;[1 1 1] Show Singleplayer Menu
  (`self.Load Singleplayer Slots`)
  (`/Engine/EditorBlueprintResources/StandardMacros.IsValid` (`self.SinglepalyerMenu`)
    (:`Is Valid`
      _)
    (:`Is Not Valid`
      (bind _returnvalue (`|CreateWidget` "/Game/Todelete/SimpleMenuUI/UI/Widgets/MenuWidgets/Widget_SingleplayerMenu.Widget_SingleplayerMenu_C" (`GameplayStatics.GetPlayerController` 0)))
      (bind _output_get (set `self.SinglepalyerMenu` _returnvalue))))
  (`UserWidget.AddToViewport` _output_get 0))

(event `self.HandleTravelError`
  (params (FailureType :type "ETravelFailure Enum" :default "NoLevel"))
  ;[1 0.09167 0 1 42] Multiplayer Only Events
  ;;[1 1 1] On Travel Error
  (`self.DisplayErrorMessage` (`|GetEnumeratorNameAsString` FailureType)))

(event `Show Load Game Menu`
  ;[0 0.5457 1 1 42] Widegts & Menu Items
  ;;[1 1 1] Show Load Game Menu
  (`/Engine/EditorBlueprintResources/StandardMacros.IsValid` (`self.LoadGameMenu`)
    (:`Is Valid`
      _)
    (:`Is Not Valid`
      (bind _returnvalue (`|CreateWidget` "/Game/Todelete/SimpleMenuUI/UI/Widgets/MenuWidgets/Widget_LoadGameMenu.Widget_LoadGameMenu_C" (`GameplayStatics.GetPlayerController` 0)))
      (bind _output_get (set `self.LoadGameMenu` _returnvalue))))
  (`UserWidget.AddToViewport` _output_get 0))

(event `Show Multiplayer Menu`
  ;[0 0.5457 1 1 42] Widegts & Menu Items
  ;;[1 1 1] Show Multiplayer Menu
  (`/Engine/EditorBlueprintResources/StandardMacros.IsValid` (`self.Multiplayer Menu`)
    (:`Is Valid`
      _)
    (:`Is Not Valid`
      (bind _returnvalue (`|CreateWidget` "/Game/Todelete/SimpleMenuUI/UI/Widgets/MenuWidgets/Widget_MultiplayerMenu.Widget_MultiplayerMenu_C" (`GameplayStatics.GetPlayerController` 0)))
      (bind _output_get (set `self.Multiplayer Menu` _returnvalue))))
  (`UserWidget.AddToViewport` _output_get 0))

(event `Show Server Browser`
  ;[0 0.5457 1 1 42] Widegts & Menu Items
  ;;[1 1 1] Show Server Browser
  (`/Engine/EditorBlueprintResources/StandardMacros.IsValid` (`self.Server Browser`)
    (:`Is Valid`
      _)
    (:`Is Not Valid`
      (bind _returnvalue (`|CreateWidget` "/Game/Todelete/SimpleMenuUI/UI/Widgets/MenuWidgets/Widget_ServerBrowser.Widget_ServerBrowser_C" (`GameplayStatics.GetPlayerController` 0)))
      (bind _output_get (set `self.Server Browser` _returnvalue))))
  (`UserWidget.AddToViewport` _output_get 0))

(event `Show Join Menu`
  ;[0 0.5457 1 1 42] Widegts & Menu Items
  ;;[1 1 1] Show Join Menu
  (`/Engine/EditorBlueprintResources/StandardMacros.IsValid` (`self.Join Menu`)
    (:`Is Valid`
      _)
    (:`Is Not Valid`
      (bind _returnvalue (`|CreateWidget` "/Game/Todelete/SimpleMenuUI/UI/Widgets/MenuWidgets/Widget_JoinMenu.Widget_JoinMenu_C" (`GameplayStatics.GetPlayerController` 0)))
      (bind _output_get (set `self.Join Menu` _returnvalue))))
  (`UserWidget.AddToViewport` _output_get 0))

(event `Show Loading Screen`
  ;[0 0.5457 1 1 42] Widegts & Menu Items
  ;;[1 1 1] Show Loading Screen
  (`/Engine/EditorBlueprintResources/StandardMacros.IsValid` (`self.Loading Screen`)
    (:`Is Valid`
      _)
    (:`Is Not Valid`
      (bind _returnvalue (`|CreateWidget` "/Game/Todelete/SimpleMenuUI/UI/Widgets/MenuWidgets/Widget_LoadingScreen.Widget_LoadingScreen_C" (`GameplayStatics.GetPlayerController` 0)))
      (bind _output_get (set `self.Loading Screen` _returnvalue))))
  (`UserWidget.AddToViewport` _output_get 0))

(event `Show Settings Menu`
  ;[0 0.5457 1 1 42] Widegts & Menu Items
  ;;[1 1 1] Show Settings Menu
  (`/Engine/EditorBlueprintResources/StandardMacros.IsValid` (`self.SettingsMenu`)
    (:`Is Valid`
      _)
    (:`Is Not Valid`
      (bind _returnvalue (`|CreateWidget` "/Game/Todelete/SimpleMenuUI/UI/Widgets/MenuWidgets/Widget_SettingsMenu.Widget_SettingsMenu_C" (`GameplayStatics.GetPlayerController` 0)))
      (bind _output_get (set `self.SettingsMenu` _returnvalue))))
  (`UserWidget.AddToViewport` _output_get 0))

(event `Quit Game`
  ;[0 0.5457 1 1 42] Widegts & Menu Items
  ;;[1 1 1] Quit Game
  (`KismetSystemLibrary.QuitGame` (`GameplayStatics.GetPlayerController` 0) "Quit"))

(fn `Apply Action Control Settings`
  (params (`Axis Mapping Name` :type Name) (`Axis Key Bindigs` :type "Array of InputActionKeyMapping Structure"))
  (bind _returnvalue (`InputSettings.GetInputSettings`))
  (for _array_element (`InputSettings.GetActionMappingByName` _returnvalue `Axis Mapping Name`)
    (`InputSettings.RemoveActionMapping` _returnvalue _array_element false)
    (`KismetSystemLibrary.PrintString` "Remove" true true (struct :`R` 1.0 :`B` 0.206346 :`A` 1.0)))
  (for _array_element_2 `Axis Key Bindigs`
    (`InputSettings.AddActionMapping` _returnvalue (make `InputActionKeyMapping` `Axis Mapping Name` false false false false (`.Key` (break `InputActionKeyMapping` _array_element_2))) true)
    (`KismetSystemLibrary.PrintString` "add" true true (struct :`R` 0.373423 :`G` 1.0 :`A` 1.0))))

(fn `Apply Audio Setting`
  (params (Master :type "Float (double-precision)") (SFX :type "Float (double-precision)") (Dialog :type "Float (double-precision)") (Soundtrack :type "Float (double-precision)") (Ambient :type "Float (double-precision)"))
  (locals (`Sound Mix` :type "SoundMix Object Reference" :default "SoundMix'/Game/Todelete/SimpleMenuUI/Audio/SoundMix_Master.SoundMix_Master'"))
  (bind _sound_mix (`local.Sound Mix`))
  (`GameplayStatics.SetSoundMixClassOverride` _sound_mix "/Game/Todelete/SimpleMenuUI/Audio/SoundClasses/SoundClass_Master.SoundClass_Master" Master)
  (`GameplayStatics.SetSoundMixClassOverride` _sound_mix "/Game/Todelete/SimpleMenuUI/Audio/SoundClasses/SoundClass_SFX.SoundClass_SFX" SFX)
  (`GameplayStatics.SetSoundMixClassOverride` _sound_mix "/Game/Todelete/SimpleMenuUI/Audio/SoundClasses/SoundClass_Dialog.SoundClass_Dialog" Dialog)
  (`GameplayStatics.SetSoundMixClassOverride` _sound_mix "/Game/Todelete/SimpleMenuUI/Audio/SoundClasses/SoundClass_Soundtrack.SoundClass_Soundtrack" Soundtrack)
  (`GameplayStatics.SetSoundMixClassOverride` _sound_mix "/Game/Todelete/SimpleMenuUI/Audio/SoundClasses/SoundClass_Ambient.SoundClass_Ambient" Ambient)
  (`GameplayStatics.PushSoundMixModifier` _sound_mix))

(fn `Apply Axis Control Settings`
  (params (`Axis Mapping Name` :type Name) (`Axis Key Bindigs` :type "Array of InputAxisKeyMapping Structure"))
  (bind _returnvalue (`InputSettings.GetInputSettings`))
  (for _array_element (`InputSettings.GetAxisMappingByName` _returnvalue `Axis Mapping Name`)
    (`InputSettings.RemoveAxisMapping` _returnvalue _array_element false))
  (for _array_element_2 `Axis Key Bindigs`
    (bind (_axisname _scale _key) (break `InputAxisKeyMapping` _array_element_2))
    (`InputSettings.AddAxisMapping` _returnvalue (make `InputAxisKeyMapping` `Axis Mapping Name` _scale _key) true)))

(fn `Generate Server Name`
  (returns (`Return Value` :type Text))
  (return (`KismetTextLibrary.Conv_StringToText` (`KismetGuidLibrary.Conv_GuidToString` (`KismetGuidLibrary.NewGuid`)))))

(fn `Get Advanced Graphics Info`
  (returns (Gamma :type "Float (double-precision)"))
  (return (`.Gamma_12_FCAE21834217136AA1942B9FEDD633D5` (break `/Game/Todelete/SimpleMenuUI/Blueprints/Global/Struct_AdvancedGraphicsInfo` (`self.AdvancedGraphicsInfo`)))))

(fn `Get Audio Info`
  (returns (`Master Volume` :type "Float (double-precision)") (`SFX Volume` :type "Float (double-precision)") (`Dialog Volume` :type "Float (double-precision)") (`Soundtrack Volume` :type "Float (double-precision)") (`Ambient Volume` :type "Float (double-precision)"))
  (bind (_audioinfo_mastervolume _audioinfo_sfxvolume _audioinfo_dialogvolume _audioinfo_soundtrackvolume _audioinfo_ambientvolume) (break `/Game/Todelete/SimpleMenuUI/Blueprints/Global/Struct_AudioInfo` (`self.AudioInfo`)))
  (return _audioinfo_mastervolume _audioinfo_sfxvolume _audioinfo_dialogvolume _audioinfo_soundtrackvolume _audioinfo_ambientvolume))

(fn `Get Control Info`
  (returns (MoveForward :type "Array of InputAxisKeyMapping Structure") (MoveRight :type "Array of InputAxisKeyMapping Structure") (Jump :type "Array of InputActionKeyMapping Structure") (InvertMouseY :type Boolean) (Fire :type "Array of InputActionKeyMapping Structure") (DashAction :type "Array of InputActionKeyMapping Structure") (Hat :type "Array of InputActionKeyMapping Structure") (Crouch :type "Array of InputActionKeyMapping Structure") (WeaponMode :type "Array of InputActionKeyMapping Structure") (CancelHat :type "Array of InputActionKeyMapping Structure"))
  (bind (_moveforward _moveright _jump _invertmousey _fire _dashaction _hat _crouch _weaponmode _cancelhat) (break `/Game/Todelete/SimpleMenuUI/Blueprints/Global/Struct_ControlInfo` (`self.ControlInfo`)))
  (return _moveforward _moveright _jump _invertmousey _fire _dashaction _hat _crouch _weaponmode _cancelhat))

(fn `Get Gameplay Info`
  (returns (`Return H-Sens` :type Integer) (`Return V-Sens` :type Integer) (FOV :type "Float (double-precision)"))
  (bind (_v_sens _h_sens _fov) (break `/Game/Todelete/SimpleMenuUI/Blueprints/Global/Struct_GameplayInfo` (`self.GameplayInfo`)))
  (return (`KismetMathLibrary.FTrunc` (* _h_sens 10.0)) (`KismetMathLibrary.FTrunc` (* _v_sens 10.0)) _fov))

(fn `Get Singleplayer Info`
  (returns (SingleplayerSlotsInfo :type "Array of /Game/Todelete/SimpleMenuUI/Blueprints/Global/Struct_SingleplayerSlot Structure") (LastUsedSingleplayerSlotIDX :type Integer))
  (return (`self.SingleplayerSlotsInfo`) (`self.LastUsedSingleplayerSlotIDX`)))

(fn `Load Game Object`
  (params (SlotName :type String))
  (returns (ReturnValue :type "SaveGame Object Reference"))
  (bind _returnvalue (`GameplayStatics.DoesSaveGameExist` SlotName))
  (if _returnvalue
    (bind _returnvalue_2 (`GameplayStatics.LoadGameFromSlot` SlotName))
    (return _returnvalue_2)
    (else
      (`KismetSystemLibrary.PrintString` (`KismetStringLibrary.Concat_StrStr` "INFO: " "Save Game - " SlotName " - dose not exist"))
      (return null))))

(fn `Load Singleplayer Slots`
  (bind _returnvalue (`self.Load Game Object` (`self.SingleplayerSlot`)))
  (bind _asgame_object_singleplayer_save_slots (cast `/Game/Todelete/SimpleMenuUI/Blueprints/SaveFiles/GameObject_SingleplayerSaveSlots` _returnvalue))
  (set `self.SingleplayerSlotsInfo` (`/Game/Todelete/SimpleMenuUI/Blueprints/SaveFiles/GameObject_SingleplayerSaveSlots.SingleplayerSlots` _asgame_object_singleplayer_save_slots))
  (set `self.LastUsedSingleplayerSlotIDX` (`/Game/Todelete/SimpleMenuUI/Blueprints/SaveFiles/GameObject_SingleplayerSaveSlots.LastUsedSlotIDX` _asgame_object_singleplayer_save_slots)))

(fn `Remove from Slots`
  (params (IDX :type Integer))
  (`KismetArrayLibrary.Array_Remove` (`self.SingleplayerSlotsInfo`) IDX)
  (if (== IDX (`self.LastUsedSingleplayerSlotIDX`))
    (set `self.LastUsedSingleplayerSlotIDX` -1)))

(fn `Save Game Object`
  (bind _returnvalue (`GameplayStatics.CreateSaveGameObject` "/Game/Todelete/SimpleMenuUI/Blueprints/SaveFiles/GameObject_SettingsSaveFile.GameObject_SettingsSaveFile_C"))
  (set `/Game/Todelete/SimpleMenuUI/Blueprints/SaveFiles/GameObject_SettingsSaveFile.AudioInfo` (`self.AudioInfo`) _returnvalue)
  (set `/Game/Todelete/SimpleMenuUI/Blueprints/SaveFiles/GameObject_SettingsSaveFile.GameplayInfo` (`self.GameplayInfo`) _returnvalue)
  (set `/Game/Todelete/SimpleMenuUI/Blueprints/SaveFiles/GameObject_SettingsSaveFile.ControlInfo` (`self.ControlInfo`) _returnvalue)
  (set `/Game/Todelete/SimpleMenuUI/Blueprints/SaveFiles/GameObject_SettingsSaveFile.GraphicsInfo` (`self.AdvancedGraphicsInfo`) _returnvalue)
  (`GameplayStatics.SaveGameToSlot` _returnvalue (`self.GameObjectSlot`)))

(fn `Save Singleplayer Slots`
  (locals (`Save Game Object Temp` :type "/Game/Todelete/SimpleMenuUI/Blueprints/SaveFiles/GameObject_SingleplayerSaveSlots Object Reference"))
  (bind _returnvalue (`GameplayStatics.CreateSaveGameObject` "/Game/Todelete/SimpleMenuUI/Blueprints/SaveFiles/GameObject_SingleplayerSaveSlots.GameObject_SingleplayerSaveSlots_C"))
  (set `/Game/Todelete/SimpleMenuUI/Blueprints/SaveFiles/GameObject_SingleplayerSaveSlots.SingleplayerSlots` (`self.SingleplayerSlotsInfo`) _returnvalue)
  (set `/Game/Todelete/SimpleMenuUI/Blueprints/SaveFiles/GameObject_SingleplayerSaveSlots.LastUsedSlotIDX` (`self.LastUsedSingleplayerSlotIDX`) _returnvalue)
  (`GameplayStatics.SaveGameToSlot` _returnvalue (`self.SingleplayerSlot`)))

(fn `Set Advanced Graphics Info`
  (params (Gamma :type "Float (double-precision)"))
  (set `self.AdvancedGraphicsInfo` (make `/Game/Todelete/SimpleMenuUI/Blueprints/Global/Struct_AdvancedGraphicsInfo` Gamma))
  (return))

(fn `Set Audio Info`
  (params (`Master Volume` :type "Float (double-precision)") (`SFX Volume` :type "Float (double-precision)") (`Dialog Volume` :type "Float (double-precision)") (`Soundtrack Volume` :type "Float (double-precision)") (`Ambient Volume` :type "Float (double-precision)"))
  (set `self.AudioInfo` (make `/Game/Todelete/SimpleMenuUI/Blueprints/Global/Struct_AudioInfo` `Master Volume` `SFX Volume` `Dialog Volume` `Soundtrack Volume` `Ambient Volume`)))

(fn `Set Control Info`
  (params (MoveForward :type "Array of InputAxisKeyMapping Structure") (MoveRight :type "Array of InputAxisKeyMapping Structure") (Jump :type "Array of InputActionKeyMapping Structure") (InvertMouseY :type Boolean) (Fire :type "Array of InputActionKeyMapping Structure") (DashAction :type "Array of InputActionKeyMapping Structure") (Hat :type "Array of InputActionKeyMapping Structure") (Crouch :type "Array of InputActionKeyMapping Structure") (WeaponMode :type "Array of InputActionKeyMapping Structure") (CancelHat :type "Array of InputActionKeyMapping Structure"))
  (set `self.ControlInfo` (make `/Game/Todelete/SimpleMenuUI/Blueprints/Global/Struct_ControlInfo` MoveForward MoveRight Jump InvertMouseY Fire DashAction Hat Crouch WeaponMode CancelHat))
  (`self.Apply Axis Control Settings` "MoveForward" MoveForward)
  (`self.Apply Axis Control Settings` "MoveRight" MoveRight)
  (`self.Apply Action Control Settings` "Jump" Jump)
  (`self.Apply Action Control Settings` "Fire" Fire)
  (`self.Apply Action Control Settings` "DashAction" DashAction)
  (`self.Apply Action Control Settings` "Hat" Hat)
  (`self.Apply Action Control Settings` "Crouch" Crouch)
  (`self.Apply Action Control Settings` "WeaponMode" WeaponMode)
  (`self.Apply Action Control Settings` "CancelHat" CancelHat))

(fn `Set Gameplay Info`
  (params (`H-Sens` :type Integer) (`V-Sens` :type Integer) (FOV :type "Float (double-precision)"))
  (set `self.GameplayInfo` (make `/Game/Todelete/SimpleMenuUI/Blueprints/Global/Struct_GameplayInfo` (* `V-Sens` 0.1) (* `H-Sens` 0.1) FOV))
  (return))

(fn `Update Slot`
  (params (Transform :type "Transform Structure"))
  (`KismetArrayLibrary.Array_Set` (`self.SingleplayerSlotsInfo`) (`self.LastUsedSingleplayerSlotIDX`) (make `/Game/Todelete/SimpleMenuUI/Blueprints/Global/Struct_SingleplayerSlot` (`.LevelName_2_57DA91F74DF6A44188F69FAB34AE3C68` (break `/Game/Todelete/SimpleMenuUI/Blueprints/Global/Struct_SingleplayerSlot` (`|GetArrayItem` (`self.SingleplayerSlotsInfo`) (`self.LastUsedSingleplayerSlotIDX`)))) Transform (`KismetMathLibrary.UtcNow`) false))
  (`self.Save Singleplayer Slots`))