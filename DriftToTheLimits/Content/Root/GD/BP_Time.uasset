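; BP_Time is a stopwatch actor that tracks elapsed minutes, seconds and milliseconds from BeginPlay.
; A looping 0.001-second timer increments the millisecond counter and rolls it into seconds and minutes, counting timer firings rather than reading a clock.
; SaveTime passes the values to the object returned by GetGIDTTS, while ResetTime zeroes them and GetTime returns them.
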(event `self.ReceiveBeginPlay`
  (`KismetSystemLibrary.K2_SetTimerDelegate` (delegate `CustomEvent_0`) 0.001 true))

(event `CustomEvent_0`
  (bind _output_get (set `self.miliSeconds` (+ (`self.miliSeconds`) 1.0)))
  (if (> _output_get 999.0)
    (set `self.miliSeconds` 0.0)
    (bind _result (`/Engine/EditorBlueprintResources/StandardMacros.IncrementInt` (`self.Seconds`))
      (:`  `
        (if (> _result 59)
          (set `self.Seconds` 0)
          (`/Engine/EditorBlueprintResources/StandardMacros.IncrementInt` (`self.Minutes`)))))))

(fn `getTime`
  (returns (M :type Integer) (S :type Integer) (MS :type "Float (double-precision)"))
  (return (`self.Minutes`) (`self.Seconds`) (`self.miliSeconds`)))

(fn `resetTime`
  (set `self.miliSeconds` 0.0)
  (set `self.Seconds` 0)
  (set `self.Minutes` 0))

(fn `saveTime`
  (`/Game/Root/GD/MyGameInstance.SetTime` (`/Game/Root/GD/MyFunction.Get_GIDTTS`) (`self.Minutes`) (`self.Seconds`) (`self.miliSeconds`)))

(fn `UserConstructionScript`)