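; BP_Ghost is a ghost car actor that replays a recorded drive from SGhostData.
; Each Tick it applies the transform and mesh rotation stored at the current Steps index, advancing one sample per frame rather than by elapsed time.
; Two spark effects, activated on BeginPlay, are shown or hidden from the recorded drift flag.
; When no further sample exists, it prints an end message and destroys itself.
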(event `self.ReceiveBeginPlay`
  (`ActorComponent.Activate` (`self.Spark_L`) false)
  (`ActorComponent.Activate` (`self.Spark_R`) false))

(event `self.ReceiveTick`
  (params (DeltaSeconds :type "Float (single-precision)"))
  (bind (_s_ghost_data_transform _s_ghost_data_meshrotation _s_ghost_data_isdrifting) (break `/Game/Root/GD/Ghost/S_GhostData` (`self.S Ghost Data`)))
  (`self.K2_SetActorTransform` (`|GetArrayItem` _s_ghost_data_transform (`self.Steps`)) true)
  (`SceneComponent.K2_SetRelativeRotation` (`self.NewCar_Mesh`) (`|GetArrayItem` _s_ghost_data_meshrotation (`self.Steps`)) false false)
  (`SceneComponent.SetHiddenInGame` (`self.Spark_L`) (not (`|GetArrayItem` _s_ghost_data_isdrifting (`self.Steps`))) false)
  (`SceneComponent.SetHiddenInGame` (`self.Spark_R`) (not (`|GetArrayItem` _s_ghost_data_isdrifting (`self.Steps`))) false)
  (if (`KismetArrayLibrary.Array_IsValidIndex` _s_ghost_data_transform (+ (`self.Steps`) 1))
    (`/Engine/EditorBlueprintResources/StandardMacros.IncrementInt` (`self.Steps`))
    (else
      (`KismetSystemLibrary.PrintString` "End Recording")
      (`self.K2_DestroyActor`))))

(fn `UserConstructionScript`
  (`parent.UserConstructionScript`))