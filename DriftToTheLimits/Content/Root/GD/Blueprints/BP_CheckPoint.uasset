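; Racing checkpoint with a resizable trigger box that tracks car progress and laps, ignoring ghost cars.
; Each overlap sets the car's restart transform and logs a passed checkpoint; Start checkpoints also register the car.
; The End checkpoint requires enough passes to save the lap time and advance the lap.
; After the final lap it sets a best-time index via CheckBL, ends that car's run and opens Menus once all registered cars finish.
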(event `self.Box.OnComponentBeginOverlap`
  (params (OverlappedComponent :type "PrimitiveComponent Object Reference") (OtherActor :type "Actor Object Reference") (OtherComp :type "PrimitiveComponent Object Reference") (OtherBodyIndex :type Integer) (bFromSweep :type Boolean) (SweepResult :type "HitResult Structure (by ref)"))
  (bind _as_bp_car_parent (`self.As BP Car Parent`))
  (bind _as_bp_car_parent_2 (`self.As BP Car Parent`))
  (bind _as_bp_car_parent_0 (`self.As BP Car Parent_0`))
  (bind _returnvalue (`KismetArrayLibrary.Array_Length` _as_bp_car_parent_0))
  (bind _hasfinished (`/Game/Root/GD/Player/BP_CarParent.hasFinished` (`|GetArrayItem` _as_bp_car_parent_0 2)))
  (cast `/Game/Root/GD/Ghost/BP_Ghost` OtherActor
    (:`CastFailed`
      (bind _asbp_car_parent (cast `/Game/Root/GD/Player/BP_CarParent` OtherActor))
      (set `self.As BP Car Parent` _asbp_car_parent)
      (set `/Game/Root/GD/Player/BP_CarParent.RestartPos` (`SceneComponent.K2_GetComponentToWorld` (`self.SkeletalMesh`)) (`self.As BP Car Parent`))
      (bind _returnvalue_2 (`GameplayStatics.GetActorOfClass` "/Game/Root/GD/Blueprints/BP_Time.BP_Time_C"))
      (set `self.Timer` _returnvalue_2)
      (`|ExecutionSequence`
        (:`then_0`
          (if (`self.Start`)
            (`KismetArrayLibrary.Array_AddUnique` (`self.As BP Car Parent_0`) (`self.As BP Car Parent`))))
        (:`then_1`
          (if (== (`self.NewVar_0`) -1)
            _
            (else
              _))
          (bind _returnvalue_3 (`KismetArrayLibrary.Array_Add` (`/Game/Root/GD/Player/BP_CarParent.ListOfCheckPointPassed` (`self.As BP Car Parent`)) true))
          (bind _output_get (set `self.NewVar_0` _returnvalue_3))
          (`KismetSystemLibrary.PrintString` (`KismetStringLibrary.Concat_StrStr` (`KismetSystemLibrary.GetDisplayName` self) " // " (`KismetStringLibrary.Conv_IntToString` _output_get)) false)
          (if (`self.IsEnd`)
            (if (> (`KismetArrayLibrary.Array_Length` (`/Game/Root/GD/Player/BP_CarParent.ListOfCheckPointPassed` (`self.As BP Car Parent`))) 25)
              (`KismetArrayLibrary.Array_Clear` (`/Game/Root/GD/Player/BP_CarParent.ListOfCheckPointPassed` (`self.As BP Car Parent`)))
              (`/Game/Root/GD/Player/BP_CarParent.SaveTime` _as_bp_car_parent_2 (`/Game/Root/GD/Player/BP_CarParent.NumberOfLaps` _as_bp_car_parent_2))
              (bind _result (`/Engine/EditorBlueprintResources/StandardMacros.IncrementInt` (`/Game/Root/GD/Player/BP_CarParent.NumberOfLaps` _as_bp_car_parent))
                (:`  `
                  (`/Game/Root/GD/Player/BP_CarParent.CallUpdateLaps` _as_bp_car_parent)
                  (`KismetSystemLibrary.PrintString` (`KismetStringLibrary.Concat_StrStr` "END TURN!!!!!" "//// LAP ==" (`KismetStringLibrary.Conv_IntToString` _result)) false true (struct :`R` 1.0 :`B` 0.098792 :`A` 1.0))
                  (if (> (`/Game/Root/GD/Player/BP_CarParent.NumberOfLaps` (`self.As BP Car Parent`)) 3)
                    (bind _idbesttime (`self.CheckBL`))
                    (set `/Game/Root/GD/Player/BP_CarParent.IdBestTime` _idbesttime (`self.As BP Car Parent`))
                    (`/Game/Root/GD/Player/BP_CarParent.EndRun` (`self.As BP Car Parent`))
                    (`KismetSystemLibrary.Delay` 3.0)
                    (`KismetSystemLibrary.PrintString` (`KismetStringLibrary.Conv_IntToString` _returnvalue) false)
                    (switch `int` _returnvalue
                      (:`1`
                        (`GameplayStatics.OpenLevel` "Menus" :!label _label))
                      (:`2`
                        (if (and (`/Game/Root/GD/Player/BP_CarParent.hasFinished` (`|GetArrayItem` _as_bp_car_parent_0)) (`/Game/Root/GD/Player/BP_CarParent.hasFinished` (`|GetArrayItem` _as_bp_car_parent_0 1))) :!label _label_2
                          (`GameplayStatics.RemovePlayer` (`GameplayStatics.GetPlayerController` 1))
                          (goto _label)))
                      (:`3`
                        (if _hasfinished
                          (goto _label_2)))
                      (:`4`
                        (if (and _hasfinished (`/Game/Root/GD/Player/BP_CarParent.hasFinished` (`|GetArrayItem` _as_bp_car_parent_0 3)))
                          (goto _label_2))))))))))))))

(fn `CheckBL`
  (returns (IdBestTime :type Integer))
  (bind _newvar_1 (`self.NewVar_1`))
  (bind _idbesttime (`self.IdBestTime`))
  (set `self.BestTime` (`|GetArrayItem` _newvar_1))
  (for (_array_element _array_index) _newvar_1
    (`KismetSystemLibrary.PrintString` (`KismetStringLibrary.Concat_StrStr` (`KismetStringLibrary.Conv_IntToString` _array_index) " // " (`KismetStringLibrary.Conv_DoubleToString` _array_element)) false)
    (bind _returnvalue (+ _array_index 1))
    (if (`KismetArrayLibrary.Array_IsValidIndex` _newvar_1 _returnvalue)
      (if (not (< (`self.BestTime`) (`|GetArrayItem` _newvar_1 _returnvalue)))
        (set `self.BestTime` _array_element)
        (set `self.IdBestTime` _returnvalue))))
  (`KismetSystemLibrary.PrintString` (`KismetStringLibrary.Conv_IntToString` _idbesttime) false)
  (return _idbesttime))

(fn `UserConstructionScript`
  (`BoxComponent.SetBoxExtent` (`self.Box`) (`self.In Box Extent`) true))