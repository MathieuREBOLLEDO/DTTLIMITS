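; BP_GhostManager spawns a replay ghost from saved data when play begins.
; It picks a save slot from the GhostToPlay selection (test, player or developer ghost) and loads it as SG_Ghost if that slot exists.
; It then spawns BP_Ghost at the first recorded transform and passes it the saved GhostData.
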(event `self.ReceiveBeginPlay`
  (bind _returnvalue (select `/Game/Root/GD/Ghost/E_GhostName` (`self.GhostToPlay`) :`NewEnumerator0` "Test_0" :`NewEnumerator1` "GhostP" :`NewEnumerator2` "GhostDev"))
  (bind _ghostdata (`/Game/Root/GD/Ghost/SG_Ghost.GhostData` (`self.SG_Instance`)))
  (bind _returnvalue_2 (`GameplayStatics.DoesSaveGameExist` _returnvalue))
  (if _returnvalue_2
    (bind _returnvalue_3 (`GameplayStatics.LoadGameFromSlot` _returnvalue))
    (bind _assg_ghost (cast `/Game/Root/GD/Ghost/SG_Ghost` _returnvalue_3))
    (set `self.SG_Instance` _assg_ghost)
    (`|SpawnActorFromClass` "/Game/Root/GD/Ghost/BP_Ghost.BP_Ghost_C" (`|GetArrayItem` (`.Transform_3_818CB9BA439A5230BB81AC82524E9CD3` (break `/Game/Root/GD/Ghost/S_GhostData` _ghostdata))) "Undefined" "OverrideRootScale" null _ghostdata 0 1 null)))

(fn `UserConstructionScript`)