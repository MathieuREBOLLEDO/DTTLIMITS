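; BP_Tool_PowerCrate is a spline-based placement tool that populates the level with BP_Energy actors.
; On BeginPlay it spawns one BP_Energy at the world location of each spline point, ignoring collisions.
; The Construction Script does nothing; its segmented mesh-along-spline logic is disconnected, leaving the start and end position/tangent helper functions used only by that dead code.
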(event `self.ReceiveBeginPlay`
  (bind _spline (`self.Spline`))
  (for _index (range (`SplineComponent.GetNumberOfSplinePoints` _spline))
    (`|SpawnActorFromClass` "/Game/Root/Levels/Levels_Obstacle/Energy/BP_Energy.BP_Energy_C" (`KismetMathLibrary.MakeTransform` (`SplineComponent.GetLocationAtSplinePoint` _spline _index "World")) "AlwaysSpawn" "OverrideRootScale" null null)))

(fn `GetEndPos/Tangent`
  (params (index :type Integer))
  (returns (Position :type "Vector Structure") (Tangent :type "Vector Structure"))
  (bind _spline (`self.Spline`))
  (bind _returnvalue (* (+ index 1) (`self.SectionLength`)))
  (return (`SplineComponent.GetLocationAtDistanceAlongSpline` _spline _returnvalue "Local") (`KismetMathLibrary.ClampVectorSize` (`SplineComponent.GetTangentAtDistanceAlongSpline` _spline _returnvalue "Local") 0.0 (`self.SectionLength`))))

(fn `GetStarPos/Tangent`
  (params (index :type Integer))
  (returns (Position :type "Vector Structure") (Tangent :type "Vector Structure"))
  (bind _spline (`self.Spline`))
  (bind _returnvalue (* index (`self.SectionLength`)))
  (return (`SplineComponent.GetLocationAtDistanceAlongSpline` _spline _returnvalue "Local") (`KismetMathLibrary.ClampVectorSize` (`SplineComponent.GetTangentAtDistanceAlongSpline` _spline _returnvalue "Local") 0.0 (`self.SectionLength`))))

(fn `UserConstructionScript`)