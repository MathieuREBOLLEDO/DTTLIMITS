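; Race position tracker that finds each non-ghost car's place along a track spline and drives the solo or multiplayer progress map.
; Looping timers set each car's nearest spline-point index, then score it as laps × 100 plus that index.
; Repeated max searches rank only the top car, plus second in multiplayer.
; Map sliders read a counter incremented on each score change, scaled to a hard-coded point and lap count.
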(event `CheckPos`
  (bind _posofplayers (`self.PosOfPlayers`))
  (bind _posofplayers_2 (`self.PosOfPlayers`))
  (bind _indexofmaxvalue (`KismetMathLibrary.MaxOfIntArray` _posofplayers_2))
  (bind _indexofmaxvalue_2 (`KismetMathLibrary.MaxOfIntArray` _posofplayers))
  (for (_array_element _array_index) (`self.List Of Player`)
    (`KismetArrayLibrary.Array_Set` (`self.PosOfPlayers`) _array_index (+ (* (`/Game/Root/GD/Player/BP_CarParent.NumberOfLaps` _array_element) 100) (`/Game/Root/GD/Player/BP_CarParent.IdPos` _array_element)))
    (bind _output (`|GetArrayItem` (`self.PosOfPlayers`) _array_index))
    (if (!= (`|GetArrayItem` (`self.PosOfPlayersTmp`) _array_index) _output)
      (`KismetArrayLibrary.Array_Set` (`self.PosOfPlayersTmp`) _array_index _output)
      (`/Engine/EditorBlueprintResources/StandardMacros.IncrementInt` (`|GetArrayItem` (`self.CurrentPos`) _array_index))))
  (set `self.Player Pos` 0)
  (set `/Game/Root/GD/Player/BP_CarParent.PlayerPos` (`self.Player Pos`) (`|GetArrayItem` (`self.List Of Player`) _indexofmaxvalue))
  (`KismetArrayLibrary.Array_Set` _posofplayers_2 _indexofmaxvalue)
  (if (!= (`/Game/Root/GD/MyGameInstance.NumberOfPlayer` (`/Game/Root/GD/MyFunction.Get_GIDTTS`)) 0)
    (`/Engine/EditorBlueprintResources/StandardMacros.IncrementInt` (`self.Player Pos`)
      (:`  `
        (set `/Game/Root/GD/Player/BP_CarParent.PlayerPos` (`self.Player Pos`) (`|GetArrayItem` (`self.List Of Player`) _indexofmaxvalue_2))
        (`KismetArrayLibrary.Array_Set` _posofplayers _indexofmaxvalue_2))))
  (for _array_element_2 (`self.List Of Player`)
    (`/Game/Root/GD/Player/BP_CarParent.CallUpdatePos` _array_element_2)))

(event `self.ReceiveBeginPlay`)

(event `Init Player`
  (bind _outactors (`GameplayStatics.GetAllActorsOfClass` "/Game/Root/GD/Player/BP_CarParent.BP_CarParent_C"))
  (for _array_element _outactors
    (cast `/Game/Root/GD/Ghost/BP_Ghost` _array_element
      (:`CastFailed`
        (`KismetArrayLibrary.Array_AddUnique` (`self.List Of Player`) _array_element)))))

(event `ShowMap`
  (bind _map_multi (`self.Map_Multi`))
  (`|ExecutionSequence`
    (:`then_0`
      (`self.Init Player`))
    (:`then_1`
      (`KismetSystemLibrary.K2_SetTimerDelegate` (delegate `Update Pos`) 0.5 true)
      (`KismetSystemLibrary.K2_SetTimerDelegate` (delegate `CheckPos`) 0.5 true)
      (if (== (`/Game/Root/GD/MyGameInstance.NumberOfPlayer` (`/Game/Root/GD/MyFunction.Get_GIDTTS`)) 0)
        (bind _returnvalue (`|CreateWidget` "/Game/Root/GD/Widget/HUD/WB_Solo.WB_Solo_C"))
        (bind _output_get (set `self.Map_Solo` _returnvalue))
        (`UserWidget.AddToViewport` _output_get 0)
        (else
          (bind _returnvalue_2 (`|CreateWidget` "/Game/Root/GD/Widget/HUD/WB_Multi.WB_Multi_C"))
          (bind _output_get_2 (set `self.Map_Multi` _returnvalue_2))
          (`UserWidget.AddToViewport` _output_get_2 0)
          (switch `int` (`/Game/Root/GD/MyGameInstance.NumberOfPlayer` (`/Game/Root/GD/MyFunction.Get_GIDTTS`))
            (:`1`
              (`Widget.SetVisibility` (`/Game/Root/GD/Widget/HUD/WB_Multi.Player_3` _map_multi) "Collapsed")
              (`Widget.SetVisibility` (`/Game/Root/GD/Widget/HUD/WB_Multi.Player_4` _map_multi) "Collapsed"))
            (:`2`
              (`Widget.SetVisibility` (`/Game/Root/GD/Widget/HUD/WB_Multi.Player_4` _map_multi) "Collapsed"))
            (:`3`
              _))))
      (`KismetSystemLibrary.K2_SetTimerDelegate` (delegate `UpdateMap`) 0.15 true))))

(event `UpdateMap`
  (bind _map_multi (`self.Map_Multi`))
  (bind _output (`|GetArrayItem` (`self.CurrentPos`)))
  (if (== (`/Game/Root/GD/MyGameInstance.NumberOfPlayer` (`/Game/Root/GD/MyFunction.Get_GIDTTS`)) 0)
    (`KismetSystemLibrary.PrintString` (`KismetStringLibrary.Conv_IntToString` _output) false)
    (`Slider.SetValue` (`/Game/Root/GD/Widget/HUD/WB_Solo.Player` (`self.Map_Solo`)) (`KismetMathLibrary.MapRangeClamped` (`KismetMathLibrary.Conv_IntToDouble` _output) 0.0 (`KismetMathLibrary.Conv_IntToDouble` (* (- 55 1) 3)) 0.0 1.0))
    (else
      (for (_array_element _array_index) (`self.List Of Player`)
        (`Slider.SetValue` (select `int` (`/Game/Root/GD/Player/BP_CarParent.Player Index` _array_element) :`0` (`/Game/Root/GD/Widget/HUD/WB_Multi.Player_1` _map_multi) :`1` (`/Game/Root/GD/Widget/HUD/WB_Multi.Player_2` _map_multi) :`2` (`/Game/Root/GD/Widget/HUD/WB_Multi.Player_3` _map_multi) :`3` (`/Game/Root/GD/Widget/HUD/WB_Multi.Player_4` _map_multi)) (`KismetMathLibrary.MapRangeClamped` (`KismetMathLibrary.Conv_IntToDouble` (`|GetArrayItem` (`self.CurrentPos`) _array_index)) 0.0 (`KismetMathLibrary.Conv_IntToDouble` (* (- 55 1) 3)) 0.0 1.0))))))

(event `Update Pos`
  (bind _spline (`self.Spline`))
  (for _array_element (`self.List Of Player`)
    (for _index (range (`SplineComponent.GetNumberOfSplinePoints` (`self.Spline`)))
      (bind (_returnvalue_x _returnvalue_y _returnvalue_z) (`KismetMathLibrary.BreakVector` (`SplineComponent.GetLocationAtSplinePoint` _spline _index "World")))
      (bind (_returnvalue_x_2 _returnvalue_y_2 _returnvalue_z_2) (`KismetMathLibrary.BreakVector` (`SplineComponent.FindLocationClosestToWorldLocation` _spline (`self.K2_GetActorLocation` _array_element) "World")))
      (if (== (`KismetMathLibrary.MakeVector` _returnvalue_x _returnvalue_y _returnvalue_z) (`KismetMathLibrary.MakeVector` _returnvalue_x_2 _returnvalue_y_2 _returnvalue_z_2) :`ErrorTolerance` 2500.0)
        (set `/Game/Root/GD/Player/BP_CarParent.IdPos` _index _array_element)
        (`KismetSystemLibrary.PrintString` (`KismetStringLibrary.Concat_StrStr` "Pos Checker $Clooses Point :" (`KismetStringLibrary.Conv_IntToString` _index)) false)
        (break)))))

(fn `GetEndPos/Tangent`
  (params (index :type Integer))
  (returns (Position :type "Vector Structure") (Tangent :type "Vector Structure"))
  (bind _spline (`self.Spline`))
  (bind _returnvalue (* (+ index 1) 0.0))
  (return (`SplineComponent.GetLocationAtDistanceAlongSpline` _spline _returnvalue "Local") (`KismetMathLibrary.ClampVectorSize` (`SplineComponent.GetTangentAtDistanceAlongSpline` _spline _returnvalue "Local"))))

(fn `GetStarPos/Tangent`
  (params (index :type Integer))
  (returns (Position :type "Vector Structure") (Tangent :type "Vector Structure"))
  (bind _returnvalue (* index 0.0))
  (bind _spline (`self.Spline`))
  (return (`SplineComponent.GetLocationAtDistanceAlongSpline` _spline _returnvalue "Local") (`KismetMathLibrary.ClampVectorSize` (`SplineComponent.GetTangentAtDistanceAlongSpline` _spline _returnvalue "Local"))))

(fn `UserConstructionScript`)