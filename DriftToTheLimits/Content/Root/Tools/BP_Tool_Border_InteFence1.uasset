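; Spline-based tool actor, named as a border fence, that lays a repeated mesh along a spline at construction time.
; The construction script adds one spline mesh per whole SectionLength, with configurable mesh, forward axis and collision.
; Helper functions supply local start and end positions and tangents clamped to section length, with Offset added to each end's X.
; An unconnected branch would derive SectionLength from actor X scale but never runs.
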(fn `GetEndPos/Tangent`
  (params (index :type Integer))
  (returns (Position :type "Vector Structure") (Tangent :type "Vector Structure"))
  (bind _spline (`self.Spline`))
  (bind _returnvalue (* (+ index 1) (`self.SectionLength`)))
  (return (`SplineComponent.GetLocationAtDistanceAlongSpline` _spline _returnvalue "Local") (`KismetMathLibrary.ClampVectorSize` (`SplineComponent.GetTangentAtDistanceAlongSpline` _spline _returnvalue "Local") 0.0 (`self.SectionLength`))))

(fn `GetStarPos/Tangent`
  (params (index :type Integer))
  (returns (Position :type "Vector Structure") (Tangent :type "Vector Structure"))
  (bind _spline (`self.Spline`))
  (bind _returnvalue (* index (`self.SectionLength`)))
  (return (`SplineComponent.GetLocationAtDistanceAlongSpline` _spline _returnvalue "Local") (`KismetMathLibrary.ClampVectorSize` (`SplineComponent.GetTangentAtDistanceAlongSpline` _spline _returnvalue "Local") 0.0 (`self.SectionLength`))))

(fn `UserConstructionScript`
  (for _index (range (`KismetMathLibrary.FTrunc` (/ (`SplineComponent.GetSplineLength` (`self.Spline`)) (`self.SectionLength`))))
    (set `self.Index` _index)
    (bind _returnvalue (`AddComponent|NODE_AddSplineMeshComponent-0`))
    (`StaticMeshComponent.SetStaticMesh` _returnvalue (`self.Mesh`))
    (`SplineMeshComponent.SetForwardAxis` _returnvalue (`self.In Forward Axis`) true)
    (`PrimitiveComponent.SetCollisionEnabled` _returnvalue "QueryAndPhysics")
    (bind (_position _tangent) (`self.GetStarPos/Tangent` (`self.Index`)))
    (bind (_position_2 _tangent_2) (`self.GetEndPos/Tangent` (`self.Index`)))
    (`SplineMeshComponent.SetStartAndEnd` _returnvalue _position _tangent (`KismetMathLibrary.MakeVector` (+ (.x _position_2) (`self.Offset`)) (.y _position_2) (.z _position_2)) _tangent_2 true)
    (`PrimitiveComponent.SetCollisionEnabled` _returnvalue (`self.CollisionType`))))