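; Lantern prop with a static mesh and point light, tinted through emissive color and intensity variables.
; The construction script builds a dynamic instance of MI_Lantern_A with those values and applies it to the mesh's first material slot.
; The same color drives the point light, while intensity affects only the material.
; The event graph holds only disabled placeholder events, so there is no runtime logic.
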(fn `UserConstructionScript`
  (bind _returnvalue (`KismetMaterialLibrary.CreateDynamicMaterialInstance` "/Game/Root/TA/Assets/Lantern/MI_Lantern_A.MI_Lantern_A"))
  (`MaterialInstanceDynamic.SetVectorParameterValue` _returnvalue "Emissive_Color" (`self.Emissive_Color`))
  (`PrimitiveComponent.SetMaterial` (`self.SM_Lantern_A`) 0 _returnvalue)
  (`MaterialInstanceDynamic.SetScalarParameterValue` _returnvalue "Emissive_Intensity" (`self.Emissive_Intensity`))
  (`PrimitiveComponent.SetMaterial` (`self.SM_Lantern_A`) 0 _returnvalue)
  (`LightComponent.SetLightColor` (`self.PointLight`) (`self.Emissive_Color`) true))