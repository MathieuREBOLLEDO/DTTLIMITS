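; Road-building tool Blueprint that lays spline meshes along a spline at construction time.
; The construction script calls CallConstructionScript, which adds collidable segments of the selected mesh every OffsetAdjust units, with tangents clamped to that length and roll taken from the spline.
; SplinePointNumber entries then swap the static mesh over given segment index ranges.
; A disconnected copy of this logic remains in the construction script.
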(fn `Call ConstructionScript`
  (bind _offset_adjust (`self.Offset Adjust`))
  (bind _offset_adjust_2 (`self.Offset Adjust`))
  (bind _spline (`self.Spline`))
  (bind _spline_2 (`self.Spline`))
  (for _index (range (+ (`KismetMathLibrary.FTrunc` (/ (`SplineComponent.GetSplineLength` (`self.Spline`)) (`self.Offset Adjust`))) 1))
    (bind _returnvalue (`AddComponent|NODE_AddSplineMeshComponent-1`))
    (`StaticMeshComponent.SetStaticMesh` _returnvalue (`self.Select_Mesh`))
    (`PrimitiveComponent.SetCollisionEnabled` _returnvalue "QueryAndPhysics")
    (bind _returnvalue_2 (* _index _offset_adjust_2))
    (bind _returnvalue_3 (* (+ _index 1) _offset_adjust_2))
    (`SplineMeshComponent.SetStartAndEnd` _returnvalue (`SplineComponent.GetLocationAtDistanceAlongSpline` _spline _returnvalue_2 "Local") (`KismetMathLibrary.ClampVectorSize` (`SplineComponent.GetTangentAtDistanceAlongSpline` _spline _returnvalue_2 "Local") 0.0 _offset_adjust) (`SplineComponent.GetLocationAtDistanceAlongSpline` _spline _returnvalue_3 "Local") (`KismetMathLibrary.ClampVectorSize` (`SplineComponent.GetTangentAtDistanceAlongSpline` _spline _returnvalue_3 "Local") 0.0 _offset_adjust) true)
    (bind _returnvalue_roll (`KismetMathLibrary.BreakRotator` (`SplineComponent.GetRotationAtDistanceAlongSpline` _spline_2 _returnvalue_2 "Local")))
    (`SplineMeshComponent.SetStartRoll` _returnvalue _returnvalue_roll true)
    (bind _returnvalue_roll_2 (`KismetMathLibrary.BreakRotator` (`SplineComponent.GetRotationAtDistanceAlongSpline` _spline_2 _returnvalue_3 "Local")))
    (`SplineMeshComponent.SetEndRoll` _returnvalue _returnvalue_roll_2 true)
    (`KismetArrayLibrary.Array_AddUnique` (`self.ListOfMesh`) _returnvalue))
  (for _array_element (`self.Spline Point Number`)
    (for _index_2 (range (`KismetMathLibrary.FTrunc` (.x (break `/Game/Root/TA/BP/Road_Elements/Road_BP/S_RoadArrayNew` _array_element))) (+ (`KismetMathLibrary.FTrunc` (.y (break `/Game/Root/TA/BP/Road_Elements/Road_BP/S_RoadArrayNew` _array_element))) 1))
      (`StaticMeshComponent.SetStaticMesh` (`|GetArrayItem` (`self.ListOfMesh`) _index_2) (`.StaticMesh_11_B709AC6B4766D77C8C105C8B7C3BE9FF` (break `/Game/Root/TA/BP/Road_Elements/Road_BP/S_RoadArrayNew` _array_element))))))

(fn `NewFunction_0`
  (params (C :type "Float (double-precision)") (A :type "Float (double-precision)") (B :type "Float (double-precision)"))
  (returns (NewParam :type Boolean))
  (return (and (> C (`KismetMathLibrary.FMin` A B)) (< C (`KismetMathLibrary.FMax` A B)))))

(fn `UserConstructionScript`
  (`self.Call ConstructionScript`))