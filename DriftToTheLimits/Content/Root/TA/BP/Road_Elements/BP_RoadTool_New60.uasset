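; Road-building tool Blueprint that lays spline mesh segments along an editable spline.
; The construction script divides the spline length into OffsetAdjust-sized steps and adds a SplineMeshComponent for each, with query and physics collision.
; Each segment takes its endpoints, tangents and roll from the spline, with tangent length clamped to the step size to limit distortion.
; The event graph holds no runtime logic.
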(fn `UserConstructionScript`
  (bind _spline (`self.Spline`))
  (bind _offset_adjust (`self.Offset Adjust`))
  (bind _offset_adjust_2 (`self.Offset Adjust`))
  (bind _spline_2 (`self.Spline`))
  (for _index (range (+ (`KismetMathLibrary.FTrunc` (/ (`SplineComponent.GetSplineLength` (`self.Spline`)) (`self.Offset Adjust`))) 1))
    (bind _returnvalue (`AddComponent|NODE_AddSplineMeshComponent-0`))
    (bind _returnvalue_2 (* _index _offset_adjust))
    (bind _returnvalue_3 (* (+ _index 1) _offset_adjust))
    (`SplineMeshComponent.SetStartAndEnd` _returnvalue (`SplineComponent.GetLocationAtDistanceAlongSpline` _spline_2 _returnvalue_2 "Local") (`KismetMathLibrary.ClampVectorSize` (`SplineComponent.GetTangentAtDistanceAlongSpline` _spline_2 _returnvalue_2 "Local") 0.0 _offset_adjust_2) (`SplineComponent.GetLocationAtDistanceAlongSpline` _spline_2 _returnvalue_3 "Local") (`KismetMathLibrary.ClampVectorSize` (`SplineComponent.GetTangentAtDistanceAlongSpline` _spline_2 _returnvalue_3 "Local") 0.0 _offset_adjust_2) true)
    (bind _returnvalue_roll (`KismetMathLibrary.BreakRotator` (`SplineComponent.GetRotationAtDistanceAlongSpline` _spline _returnvalue_2 "Local")))
    (`SplineMeshComponent.SetStartRoll` _returnvalue _returnvalue_roll true)
    (bind _returnvalue_roll_2 (`KismetMathLibrary.BreakRotator` (`SplineComponent.GetRotationAtDistanceAlongSpline` _spline _returnvalue_3 "Local")))
    (`SplineMeshComponent.SetEndRoll` _returnvalue _returnvalue_roll_2 true)
    (`PrimitiveComponent.SetCollisionEnabled` _returnvalue "QueryAndPhysics")))