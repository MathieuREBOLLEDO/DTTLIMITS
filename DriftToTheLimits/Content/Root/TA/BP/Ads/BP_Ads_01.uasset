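; BP_Ads_01 is an advertisement prop that rotates three ad images on its SMAds mesh.
; From BeginPlay it sets the BFTB, LE and ED ad materials on material slot 0 in turn, waiting for the Time variable after each.
; The Again custom event calls itself after the last delay, so the cycle repeats indefinitely without Tick or a timer handle.
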(event `Again`
  (`PrimitiveComponent.SetMaterial` (`self.SM_Ads`) 0 "/Game/Root/TA/Assets/Ads/MI_Ad_BFTB.MI_Ad_BFTB" :!label _label)
  (`KismetSystemLibrary.Delay` (`self.Time`))
  (`PrimitiveComponent.SetMaterial` (`self.SM_Ads`) 0 "/Game/Root/TA/Assets/Ads/MI_Ad_LE.MI_Ad_LE")
  (`KismetSystemLibrary.Delay` (`self.Time`))
  (`PrimitiveComponent.SetMaterial` (`self.SM_Ads`) 0 "/Game/Root/TA/Assets/Ads/MI_Ad_ED.MI_Ad_ED")
  (`KismetSystemLibrary.Delay` (`self.Time`))
  (`self.Again`))

(event `self.ReceiveBeginPlay`
  (goto _label))

(fn `UserConstructionScript`)