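; BP_Ads_04 is an advertising display actor that rotates through three video ad materials on its SMAds mesh.
; On BeginPlay it applies the AD, LE and FA video materials to material slot 0 in turn, waiting Time seconds after each.
; The Again custom event calls itself after the last Delay, so the rotation repeats indefinitely without a timer or Tick.
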(event `Again`
  (`PrimitiveComponent.SetMaterial` (`self.SM_Ads`) 0 "/Game/Root/TA/Assets/Ads/MI_Ad_ADVideo.MI_Ad_ADVideo" :!label _label)
  (`KismetSystemLibrary.Delay` (`self.Time`))
  (`PrimitiveComponent.SetMaterial` (`self.SM_Ads`) 0 "/Game/Root/TA/Assets/Ads/MI_Ad_LEVideo.MI_Ad_LEVideo")
  (`KismetSystemLibrary.Delay` (`self.Time`))
  (`PrimitiveComponent.SetMaterial` (`self.SM_Ads`) 0 "/Game/Root/TA/Assets/Ads/MI_AdVideo_FA.MI_AdVideo_FA")
  (`KismetSystemLibrary.Delay` (`self.Time`))
  (`self.Again`))

(event `self.ReceiveBeginPlay`
  (goto _label))

(fn `UserConstructionScript`)