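; Tower prop Blueprint (BP_Tour_01) whose cloth pieces are tinted with a per-instance Color.
; The Construction Script creates a dynamic material instance for each of the five cloth meshes, four from the A cloth material and one from the B.
; Each instance gets Color as its "Color" vector parameter and is applied to slot 0, while the event graph holds no logic.
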(fn `UserConstructionScript`
  (bind _sm_cloth_tour_01_a (`self.SM_Cloth_Tour_01_A`))
  (bind _sm_cloth_tour_01_b (`self.SM_Cloth_Tour_01_B`))
  (bind _sm_cloth_tour_01_a1 (`self.SM_Cloth_Tour_01_A1`))
  (bind _sm_cloth_tour_01_a2 (`self.SM_Cloth_Tour_01_A2`))
  (bind _sm_cloth_tour_01_a3 (`self.SM_Cloth_Tour_01_A3`))
  (bind _returnvalue (`PrimitiveComponent.CreateDynamicMaterialInstance` _sm_cloth_tour_01_a 0 "/Game/Root/TA/Assets/Tours/Tour_01/MI_Cloth_Tour_01_A.MI_Cloth_Tour_01_A" "None"))
  (`MaterialInstanceDynamic.SetVectorParameterValue` _returnvalue "Color" (`self.Color`))
  (`PrimitiveComponent.SetMaterial` _sm_cloth_tour_01_a 0 _returnvalue)
  (bind _returnvalue_2 (`PrimitiveComponent.CreateDynamicMaterialInstance` _sm_cloth_tour_01_a1 0 "/Game/Root/TA/Assets/Tours/Tour_01/MI_Cloth_Tour_01_A.MI_Cloth_Tour_01_A" "None"))
  (`MaterialInstanceDynamic.SetVectorParameterValue` _returnvalue_2 "Color" (`self.Color`))
  (`PrimitiveComponent.SetMaterial` _sm_cloth_tour_01_a1 0 _returnvalue_2)
  (bind _returnvalue_3 (`PrimitiveComponent.CreateDynamicMaterialInstance` _sm_cloth_tour_01_a2 0 "/Game/Root/TA/Assets/Tours/Tour_01/MI_Cloth_Tour_01_A.MI_Cloth_Tour_01_A" "None"))
  (`MaterialInstanceDynamic.SetVectorParameterValue` _returnvalue_3 "Color" (`self.Color`))
  (`PrimitiveComponent.SetMaterial` _sm_cloth_tour_01_a2 0 _returnvalue_3)
  (bind _returnvalue_4 (`PrimitiveComponent.CreateDynamicMaterialInstance` _sm_cloth_tour_01_a3 0 "/Game/Root/TA/Assets/Tours/Tour_01/MI_Cloth_Tour_01_A.MI_Cloth_Tour_01_A" "None"))
  (`MaterialInstanceDynamic.SetVectorParameterValue` _returnvalue_4 "Color" (`self.Color`))
  (`PrimitiveComponent.SetMaterial` _sm_cloth_tour_01_a3 0 _returnvalue_4)
  (bind _returnvalue_5 (`PrimitiveComponent.CreateDynamicMaterialInstance` _sm_cloth_tour_01_b 0 "/Game/Root/TA/Assets/Tours/Tour_01/MI_Cloth_Tour_01_B.MI_Cloth_Tour_01_B" "None"))
  (`MaterialInstanceDynamic.SetVectorParameterValue` _returnvalue_5 "Color" (`self.Color`))
  (`PrimitiveComponent.SetMaterial` _sm_cloth_tour_01_b 0 _returnvalue_5))